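; Game mode for the Duck Hunt level that keeps the running score and ends the level on a win.
; The Addpoints event adds incoming points to FinalScore and compares the total to WinCondition.
; Once the target is reached, a DoOnce plays the win animation on the player pawn's DuckHuntUI widget, then opens StartupMap after a short delay.
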(event `Add points`
  (params (Score :type Integer))
  ;[1 1 1] Adding score to the final score
  (set `self.Final Score` (+ Score (`self.Final Score`)))
  ;[1 1 1] Win condition = Obtain 5 or more points
  (if (>= (`self.Final Score`) (`self.Win Condition`))
    (bind _asbp_duck_hunt_pawn (cast `/Game/DuckHunt/BP_DuckHuntPawn` (`GameplayStatics.GetPlayerPawn` 0)))
    (`/Engine/EditorBlueprintResources/StandardMacros.DoOnce` false
      (:`Completed`
        (bind _duckhuntui (`/Game/DuckHunt/BP_DuckHuntPawn.DuckHuntUI` _asbp_duck_hunt_pawn))
        (`UserWidget.PlayAnimation` _duckhuntui (`/Game/DuckHunt/WBP_DuckHuntUI.Win_animation` _duckhuntui) 0.0 1 "Forward" 1.0 false)
        (`KismetSystemLibrary.Delay` 3.0)
        (`GameplayStatics.OpenLevelBySoftObjectPtr` "/Game/MainBlueprints/StartupMap.StartupMap")))))

(fn `UserConstructionScript`)