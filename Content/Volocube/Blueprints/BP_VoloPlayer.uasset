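; BP_VoloPlayer is the Volocube player character, kept between two wall limits along the world X axis.
; Each Tick it compares its X location to LocWall1 (upper) and LocWall2 (lower), snapping X back to the crossed limit while preserving Y and Z.
; An unconnected debug print shows X velocity as a fraction of the movement component's max speed.
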(event `self.ReceiveTick`
  (params (DeltaSeconds :type "Float (single-precision)"))
  (bind (_returnvalue_x _returnvalue_y _returnvalue_z) (`KismetMathLibrary.BreakVector` (`self.K2_GetActorLocation`)))
  (if (> _returnvalue_x (`self.LocWall1`))
    (`self.K2_SetActorLocation` (`KismetMathLibrary.MakeVector` (`self.LocWall1`) _returnvalue_y _returnvalue_z))
    (elif (< _returnvalue_x (`self.LocWall2`))
      (`self.K2_SetActorLocation` (`KismetMathLibrary.MakeVector` (`self.LocWall2`) _returnvalue_y _returnvalue_z)))))

(fn `UserConstructionScript`)