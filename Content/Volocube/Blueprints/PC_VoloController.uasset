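; Player controller for Volocube that handles movement and game-speed input and shows the score UI.
; On BeginPlay it registers the Volocube input mapping context and, in the same validity branch, adds the score widget to the viewport.
; IA_UP feeds movement along world X to the possessed pawn.
; Speed and Slow inputs change global time dilation while active, both returning to a slightly faster-than-real-time rate on completion.
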(event `self.ReceiveBeginPlay`
  (bind _returnvalue (pcsubsystem `EnhancedInputLocalPlayerSubsystem` (`GameplayStatics.GetPlayerController` 0)))
  (`/Engine/EditorBlueprintResources/StandardMacros.IsValid` _returnvalue
    (:`Is Valid`
      (`EnhancedInputSubsystemInterface.AddMappingContext` _returnvalue "/Game/Volocube/InputActions/IM_Volocube.IM_Volocube" 0 (struct))
      (bind _returnvalue_2 (`|CreateWidget` "/Game/Volocube/UI/WBP_Score.WBP_Score_C"))
      (`UserWidget.AddToViewport` _returnvalue_2 0))))

(event `EnhancedInput|/Game/Volocube/InputActions/IA_UP`
  (params (ActionValue :type "Float (double-precision)") (ElapsedSeconds :type "Float (double-precision)") (TriggeredSeconds :type "Float (double-precision)") (InputAction :type "InputAction Object Reference" :default "/Game/Volocube/InputActions/IA_UP.IA_UP"))
  (:`Triggered`
    (`Pawn.AddMovementInput` (`self.K2_GetPawn`) (1.0 0.0 0.0) ActionValue false)))

(event `EnhancedInput|/Game/Volocube/InputActions/IA_Speed`
  (params (ActionValue :type Boolean) (ElapsedSeconds :type "Float (double-precision)") (TriggeredSeconds :type "Float (double-precision)") (InputAction :type "InputAction Object Reference" :default "/Game/Volocube/InputActions/IA_Speed.IA_Speed"))
  (:`Triggered`
    (`GameplayStatics.SetGlobalTimeDilation` 3.0))
  (:`Completed`
    (`GameplayStatics.SetGlobalTimeDilation` 1.3)))

(event `EnhancedInput|/Game/Volocube/InputActions/IA_Slow`
  (params (ActionValue :type Boolean) (ElapsedSeconds :type "Float (double-precision)") (TriggeredSeconds :type "Float (double-precision)") (InputAction :type "InputAction Object Reference" :default "/Game/Volocube/InputActions/IA_Slow.IA_Slow"))
  (:`Triggered`
    (`GameplayStatics.SetGlobalTimeDilation` 0.5))
  (:`Completed`
    (`GameplayStatics.SetGlobalTimeDilation` 1.3)))

(fn `UserConstructionScript`)