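; Pong-style ball for Volocube that launches in a random diagonal and moves every tick through a FloatingPawnMovement.
; Overlaps with walls scale X velocity by BallSpeed; player hits scale Y and add the player's normalized X velocity as steering, with both raising max speed.
; Goal zones update the player or enemy score on the game mode, spawn a replacement ball and explosion at the starting location, then destroy this ball.
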(event `self.ReceiveBeginPlay`
  (bind _returnvalue_location (`KismetMathLibrary.BreakTransform` (`self.GetTransform`)))
  (set `self.BallVelocity` (`KismetMathLibrary.MakeVector` (select `bool` (`KismetMathLibrary.RandomBool`) :`false` -1.0 :`true` 1.0) (select `bool` (`KismetMathLibrary.RandomBool`) :`false` -1.0 :`true` 1.0)))
  (set `self.Ball Spawning Location Location` _returnvalue_location))

(event `self.ReceiveTick`
  (params (DeltaSeconds :type "Float (single-precision)"))
  (`PawnMovementComponent.AddInputVector` (`self.FloatingPawnMovement`) (`self.BallVelocity`) false))

(event `self.Collision.OnComponentBeginOverlap`
  (params (OverlappedComponent :type "PrimitiveComponent Object Reference") (OtherActor :type "Actor Object Reference") (OtherComp :type "PrimitiveComponent Object Reference") (OtherBodyIndex :type Integer) (bFromSweep :type Boolean) (SweepResult :type "HitResult Structure (by ref)"))
  (bind (_ballvelocity_x _ballvelocity_y _ballvelocity_z) (`KismetMathLibrary.BreakVector` (`self.BallVelocity`)))
  (bind (_ballvelocity_x_2 _ballvelocity_y_2 _ballvelocity_z_2) (`KismetMathLibrary.BreakVector` (`self.BallVelocity`)))
  (bind _floatingpawnmovement (`self.FloatingPawnMovement`))
  (cast `/Game/Volocube/Blueprints/BP_Wall` OtherActor
    (:`then`
      (`GameplayStatics.PlaySound2D` "/Engine/EditorSounds/Notifications/CompileStart_Cue.CompileStart_Cue" 1.0 1.0 0.0 null null)
      (set `self.BallVelocity` (`KismetMathLibrary.MakeVector` (* _ballvelocity_x_2 (`self.BallSpeed`)) _ballvelocity_y_2 _ballvelocity_z_2))
      (set `FloatingPawnMovement.MaxSpeed` (* (`MovementComponent.GetMaxSpeed` _floatingpawnmovement) (`self.SpeedMultiplier`)) _floatingpawnmovement :!label _label))
    (:`CastFailed`
      (bind _asbp_volo_player (cast `/Game/Volocube/Blueprints/BP_VoloPlayer` OtherActor)
        (:`then`
          (`GameplayStatics.PlaySound2D` "/Engine/VREditor/Sounds/UI/Drop_Item_From_ContentBrowser.Drop_Item_From_ContentBrowser" 1.0 1.0 0.0 null null)
          (bind _returnvalue_x (`KismetMathLibrary.BreakVector` (`self.GetVelocity` _asbp_volo_player)))
          (set `self.BallVelocity` (`KismetMathLibrary.MakeVector` (+ _ballvelocity_x (/ _returnvalue_x (`MovementComponent.GetMaxSpeed` (`Character.CharacterMovement` _asbp_volo_player)))) (* _ballvelocity_y (`self.BallSpeed`)) _ballvelocity_z))
          (goto _label))
        (:`CastFailed`
          (bind _asbp_goal_zone (cast `/Game/Volocube/Blueprints/BP_GoalZone` OtherActor))
          (`self.Goal` (`/Game/Volocube/Blueprints/BP_GoalZone.PlayerTargetGoal` _asbp_goal_zone))
          (`self.K2_DestroyActor`))))))

(event `Goal`
  (params (PlayerScores :type Boolean))
  (bind _asbp_gm_volocube_main (cast `/Game/Volocube/Blueprints/BP_GM_VolocubeMain` (`GameplayStatics.GetGameMode`)))
  (`/Engine/EditorBlueprintResources/StandardMacros.IncrementInt` (select `bool` PlayerScores :`false` (`/Game/Volocube/Blueprints/BP_GM_VolocubeMain.EnemyScore` _asbp_gm_volocube_main) :`true` (`/Game/Volocube/Blueprints/BP_GM_VolocubeMain.PlayerScore` _asbp_gm_volocube_main))
    (:`  `
      (`|SpawnActorFromClass` "BP_Ball_C" (`KismetMathLibrary.MakeTransform` (`self.Ball Spawning Location Location`)) "AlwaysSpawn" "MultiplyWithRoot" null null)
      (`NiagaraFunctionLibrary.SpawnSystemAttached` "/Game/RocketDefence/Niagara_Explosion.Niagara_Explosion" null "None" (`self.Ball Spawning Location Location`) (struct) "KeepWorldPosition" false true "AutoRelease")
      (`GameplayStatics.SpawnSound2D` "/Engine/EditorSounds/GamePreview/EndSimulate_Cue.EndSimulate_Cue" 1.0 1.0 0.0 null)
      (`self.K2_DestroyActor`))))

(fn `UserConstructionScript`)