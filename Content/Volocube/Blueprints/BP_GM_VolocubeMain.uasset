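; BP_GM_VolocubeMain is the main game mode for Volocube, tracking win and loss state from the player and enemy scores.
; On BeginPlay it sets a timer that fires the Winning event after one second, with no looping shown.
; Winning checks both scores independently, flagging Won when the player's score exceeds one and Lost when the enemy's is above zero, so both flags can be set.
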(event `self.ReceiveBeginPlay`
  (`KismetSystemLibrary.K2_SetTimerDelegate` (delegate `Winning`) 1.0))

(event `Winning`
  (`|ExecutionSequence`
    (:`then_0`
      (if (> (`self.PlayerScore`) 1)
        (set `self.Won` true)))
    (:`then_1`
      (if (> (`self.EnemyScore`) 0)
        (set `self.Lost` true)))))

(fn `UserConstructionScript`)